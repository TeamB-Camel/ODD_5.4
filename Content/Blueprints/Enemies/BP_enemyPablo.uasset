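; Enemy Pablo: a paper-sprite enemy with a health bar that flees when the player gets close.
; Tick syncs health to the widget, turns sprite and bar toward player and camera, and displays player distance as debug-style text.
; Fleeing picks a random room connected to the nearest BP_roomBounds and uses AIMoveTo to a random point there, guarded by IsFlee.
; It also spawns a NavigationTestingActor at a separately randomized point.
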(event Custom|runAway
  (if (not (Variables|Default|GetisFlee))
    (Variables|Default|SetisFlee true)
    (bind _outactors (Actor|GetAllActorsOfClass "/Game/Blueprints/Level/BP_roomBounds.BP_roomBounds_C"))
    (bind _asbp_room_bounds (Utilities|Casting|CastToBP_roomBounds (.ReturnValue (Actor|FindNearestActor (Transformation|GetActorLocation) _outactors)))
      (:then
        (Development|PrintString "Found Room")
        (bind _asbp_room_bounds_2 (Utilities|Casting|CastToBP_roomBounds (.OutItem (Utilities|Array|Random (Variables|/Game/Blueprints/Level/BP_roomBounds.BP_roomBounds_C|GetconnectedRooms _asbp_room_bounds)))))
        (Game|SpawnActorfromClass "/Script/NavigationSystem.NavigationTestingActor" (Math|Transform|MakeTransform (Math|Random|RandomPointinBoundingBox (.Origin (Collision|GetActorBounds _asbp_room_bounds_2 false false)) (.BoxExtent (Collision|GetActorBounds _asbp_room_bounds_2 false false))) "0, 0, 0" "1.000000,1.000000,1.000000") "Undefined" "MultiplyWithRoot" 0 0)
        (AI|AIMoveTo self (Math|Random|RandomPointinBoundingBox (.Origin (Collision|GetActorBounds _asbp_room_bounds_2 false false)) (.BoxExtent (Collision|GetActorBounds _asbp_room_bounds_2 false false))) 0 4e+01 false
          (:then
            (Development|PrintString "M;oving"))
          (:OnSuccess
            (Development|PrintString "Reached Loc")
            (Variables|Default|SetisFlee false :!label _label))
          (:OnFail
            (Development|PrintString "I am Looser")
            (goto _label))))
      (:CastFailed
        (Development|PrintString "Balls" true true "(R=0.000000,G=0.660000,B=1.000000,A=1.000000)" 1e+01)))))

(event EventBeginPlay
  (Variables|Default|SetcurHealth (Variables|Default|GetmaxHealth))
  (bind _aswbp_enemy_healthbar (Utilities|Casting|CastToWBP_enemyHealthbar (UserInterface|GetWidget (Variables|Default|GethealthBar))))
  (bind _output_get (Variables|Default|SetAs%20WBP%20Enemy%20Healthbar _aswbp_enemy_healthbar))
  (Variables|/Game/Blueprints/Interface/WBP_enemyHealthbar.WBP_enemyHealthbar_C|SetmaxHealth _output_get (Variables|Default|GetmaxHealth)))

(event EventTick
  (params (DeltaSeconds :type Float%20%28single-precision%29))
  (bind _papersprite (Variables|Default|GetPaperSprite))
  (bind _healthbar (Variables|Default|GethealthBar))
  (Utilities|FlowControl|Sequence
    (:then_0
      (Variables|/Game/Blueprints/Interface/WBP_enemyHealthbar.WBP_enemyHealthbar_C|SetcurHealth (Variables|Default|GetAs%20WBP%20Enemy%20Healthbar) (Variables|Default|GetcurHealth))
      (if (== (Utilities|GetClass (Game|GetPlayerCharacter 0)) "/Game/Blueprints/Player/BP_playerCharacter.BP_playerCharacter_C")
        (Transformation|SetWorldRotation _papersprite (Math|Rotator|MakeRotator 0.0 0.0 (+ (.yaw (Math|Rotator|FindLookatRotation (Transformation|GetWorldLocation _papersprite) (Transformation|GetActorLocation (Game|Player|GetPlayerPawn 0)))) 9e+01)) false false)
        (Transformation|SetWorldRotation _healthbar (Math|Rotator|FindLookatRotation (Transformation|GetWorldLocation _healthbar) (Transformation|GetWorldLocation (Variables|/Script/Engine.PlayerCameraManager|GetTransformComponent (Game|GetPlayerCameraManager 0)))) false false)
        (Rendering|Components|TextRender|SetText (Variables|Default|GetTextRender) (Utilities|Text|ToText(Float) (Transformation|GetDistanceTo (Game|Player|GetPlayerPawn 0)) "HalfToEven"))))
    (:then_1
      (if (and (< (Transformation|GetDistanceTo (Game|Player|GetPlayerPawn 0)) 600.1) (not (Variables|Default|GetisFlee)))
        (CallFunction|RunAway)))))

(fn ConstructionScript)