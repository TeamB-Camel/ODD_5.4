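; BP_damageNumber is a floating damage number actor that shows a Damage value as world-space text.
; On BeginPlay it picks a slightly randomized upward drift, sizes the text by damage, and sets the text one tick later.
; Each tick it turns the text to face the player character by yaw, rises with decaying speed, shrinks at an accelerating rate, and destroys itself once small.
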(event EventBeginPlay
  (bind _textrender (Variables|Default|GetTextRender))
  (bind _asbp_player_character (Utilities|Casting|CastToBP_playerCharacter (Game|GetPlayerCharacter 0)))
  (Variables|Default|SetAs%20BP%20Player%20Character _asbp_player_character)
  (Variables|Default|SetvecAscend (Math|Vector|MakeVector (Math|Random|RandomFloatinRange 0.0 0.5) (Math|Random|RandomFloatinRange 0.0 0.5) 1.0))
  (Rendering|Components|TextRender|SetWorldSize _textrender (* (+ (/ (Variables|Default|Getdamage) 1e+01) 1.0) 5e+01))
  (Utilities|FlowControl|DelayUntilNextTick)
  (Rendering|Components|TextRender|SetText _textrender (Utilities|Text|ToText(Float) (Variables|Default|Getdamage) "HalfToEven")))

(event EventTick
  (params (DeltaSeconds :type Float%20%28single-precision%29))
  (bind _returnvalue (Transformation|GetActorLocation))
  (bind _textrender (Variables|Default|GetTextRender))
  (bind _as_bp_player_character (Variables|Default|GetAs%20BP%20Player%20Character))
  (bind _returnvalue_2 (Transformation|GetActorLocation _as_bp_player_character))
  (bind _worldsize (Variables|/Script/Engine.TextRenderComponent|GetWorldSize _textrender))
  (bind _returnvalue_3 (Math|Rotator|FindLookatRotation _returnvalue _returnvalue_2))
  (Transformation|SetWorldRotation (Variables|Default|GetTextRender) (Math|Rotator|MakeRotator (.roll _returnvalue_3) 0.0 (.yaw _returnvalue_3)) false false)
  (Transformation|SetActorLocation (+ (Transformation|GetActorLocation) (* (Variables|Default|GetvecAscend) (Variables|Default|Getspd)) "") false false)
  (Variables|Default|Setspd (* (Variables|Default|Getspd) 0.965))
  (Rendering|Components|TextRender|SetWorldSize _textrender (- _worldsize (Variables|Default|GetfacShrink)))
  (Variables|Default|SetfacShrink (+ (Variables|Default|GetfacShrink) 0.03))
  (if (< _worldsize 5.0)
    (Actor|DestroyActor)))

(fn ConstructionScript)