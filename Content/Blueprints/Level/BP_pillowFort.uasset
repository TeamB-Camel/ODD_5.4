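; BP_pillowFort is a punchable pillow fort in the level that breaks down into a pillow pickup.
; It starts at max HP and loses one per bePunched call, swapping its static mesh to the array entry indexed by the remaining HP.
; At zero it spawns a BP_pickupPillow at its transform with a downward dislodge vector, then destroys itself.
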(event Custom|bePunched
  (Math|Integer|DecrementInt (Variables|Default|Gethp)
    (:%20%20
      (if (> (Variables|Default|Gethp) 0)
        (Components|StaticMesh|SetStaticMesh (Variables|Default|Getpillow_fort) (Utilities|Array|Get(acopy) (Variables|Default|GetarrayMesh) (Variables|Default|Gethp)))
        (else
          (bind _returnvalue (Game|SpawnActorfromClass "/Game/Blueprints/Player/BP_pickupPillow.BP_pickupPillow_C" (Transformation|GetActorTransform) "Undefined" "MultiplyWithRoot" 0 0))
          (Variables|/Game/Blueprints/Player/BP_pickupPillow.BP_pickupPillow_C|SetvecDislodge _returnvalue "0.000000,0.000000,-0.500000")
          (Actor|DestroyActor))))))

(event EventBeginPlay
  (Variables|Default|Sethp (Variables|Default|GethpMax)))

(fn ConstructionScript)