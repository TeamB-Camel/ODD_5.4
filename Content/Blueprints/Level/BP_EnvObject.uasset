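; BP_EnvObject is a level object with staged condition that can be sabotaged or repaired and damages the player's world health.
; On Tick, HP below zero drops a Stage and refills HP, or disables sabotage at stage zero.
; HP above max raises Stage only if it already exceeds StageMax, otherwise disabling repair.
; Every tick also subtracts WorldDamageValue from the player character's HpWorld, without delta-time scaling.
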(event EventTick
  (params (DeltaSeconds :type Float%20%28single-precision%29))
  (bind _stage (Variables|Components|Getstage))
  (bind _stage_2 (Variables|Components|Getstage))
  (Utilities|FlowControl|Sequence
    (:then_2
      ;[0.15 0.15 0.15 0.5] Decrement State
      (if (< (Variables|Components|GetHP) 0.0) ; if hp < 0
        (if (> _stage_2 0) ; if stage > 0
          (Math|Integer|DecrementInt _stage_2
            (:%20%20
              (Variables|Components|SetHP (Variables|Components|GetHPMax))))
          (else
            (Variables|Components|SetcanBeSabotaged false)))))
    (:then_3
      ;[0.15 0.15 0.15 0.5] Increment State
      (if (> (Variables|Components|GetHP) (Variables|Components|GetHPMax)) ; if hp > Max
        (if (> _stage (Variables|Components|GetstageMax)) ; if stage < Max
          (Math|Integer|IncrementInt _stage
            (:%20%20
              (Variables|Components|SetHP 0.0)))
          (else
            (Variables|Components|SetcanBeRepaired false)))))
    (:then_4
      ;[0.15 0.15 0.15 0.5] Apply World Damage
      (bind _asbp_player_character (Utilities|Casting|CastToBP_playerCharacter (Game|Player|GetPlayerPawn 0)))
      (Variables|/Game/Blueprints/Player/BP_playerCharacter.BP_playerCharacter_C|SethpWorld _asbp_player_character (- (Variables|/Game/Blueprints/Player/BP_playerCharacter.BP_playerCharacter_C|GethpWorld _asbp_player_character) (Variables|Components|GetworldDamageValue))))))

(fn ConstructionScript)