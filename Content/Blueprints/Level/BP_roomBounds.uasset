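; BP_roomBounds is a room volume actor that builds its list of connected rooms at BeginPlay.
; It queries WorldDynamic actors overlapping its StaticMesh, then queries each one's mesh for overlapping BP_roomBounds and adds those other than itself to ConnectedRooms.
; Both overlap queries pass the component's relative transform rather than its world transform.
; Debug prints report the overlap and connection counts.
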(event EventBeginPlay
  (bind _staticmesh (Variables|Default|GetStaticMesh))
  (bind _connectedrooms (Variables|Default|GetconnectedRooms))
  (bind _outactors (Collision|ComponentOverlapActors _staticmesh (Transformation|GetRelativeTransform _staticmesh) (Utilities|Array|MakeArray "ObjectTypeQuery2") 0))
  (Development|PrintString (Utilities|String|Append (Utilities|GetDisplayName self) (Utilities|String|ToString(Integer) (Utilities|Array|Length _outactors))) true true "(R=0.000000,G=0.660000,B=1.000000,A=1.000000)" 3e+01)
  (for _array_element _outactors
    (bind _outactors_2 (Collision|ComponentOverlapActors (Actor|GetComponentbyClass _array_element "/Script/Engine.StaticMeshComponent") (Transformation|GetRelativeTransform (Actor|GetComponentbyClass _array_element "/Script/Engine.StaticMeshComponent")) (Utilities|Array|MakeArray "ObjectTypeQuery2") "BP_roomBounds_C"))
    (Development|PrintString (Utilities|String|Append (Utilities|GetDisplayName self) (Utilities|String|ToString(Integer) (Utilities|Array|Length _outactors_2))) true true "(R=0.000000,G=0.660000,B=1.000000,A=1.000000)" 3e+01)
    (for _array_element_2 _outactors_2
      (if (!= _array_element_2 self)
        (Utilities|Array|Add _connectedrooms _array_element_2)))
    (Development|PrintString (Utilities|String|Append "Connected Rooms:" (Utilities|String|ToString(Integer) (Utilities|Array|Length _connectedrooms))) true true "(R=0.000000,G=0.660000,B=1.000000,A=1.000000)" 3e+01)))

(fn ConstructionScript)