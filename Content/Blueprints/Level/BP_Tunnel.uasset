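; BP_Tunnel is a level actor for a tunnel that can be toggled between blocked and open for navigation.
; Tick shows its two text renders only while the player character is within 600 units.
; The blocked event flips TunnelBlocked, changes the text renders' material and switches the NavModifier between default and null nav areas.
; Both branches set the texts' custom trace channel response to Block.
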(event Custom|blocked
  (bind _navmodifier (Variables|Default|GetNavModifier))
  (bind _textrender (Variables|Default|GetTextRender))
  (bind _textrender_2 (Variables|Default|GetTextRender))
  (if (Variables|Default|GettunnelBlocked)
    (Variables|Default|SettunnelBlocked false)
    (Rendering|Material|SetMaterial _textrender 0 "/Engine/BasicShapes/BasicShapeMaterial.BasicShapeMaterial")
    (Collision|SetCollisionResponsetoChannel _textrender "ECC_GameTraceChannel1" "ECR_Block")
    (Class|NavModifierComponent|SetAreaClass _navmodifier "/Script/NavigationSystem.NavArea_Default")
    (else
      (Variables|Default|SettunnelBlocked true)
      (Rendering|Material|SetMaterial _textrender_2 0 0)
      (Collision|SetCollisionResponsetoChannel _textrender_2 "ECC_GameTraceChannel1" "ECR_Block")
      (Class|NavModifierComponent|SetAreaClass _navmodifier "/Script/NavigationSystem.NavArea_Null"))))

(event EventTick
  (params (DeltaSeconds :type Float%20%28single-precision%29))
  (bind _textrender1 (Variables|Default|GetTextRender1))
  (bind _asbp_player_character (Utilities|Casting|CastToBP_playerCharacter (Game|Player|GetPlayerPawn 0)))
  (if (< (Transformation|GetDistanceTo self _asbp_player_character) 6e+02)
    (Rendering|SetVisibility _textrender1 true false)
    (else
      (Rendering|SetVisibility _textrender1 false false))))

(fn ConstructionScript)