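; Minigame hand pawn that, when possessed, picks a random minigame and spawns its pieces, apparently still work in progress.
; It caches the instigating player character, then spawns a small grabber at a random point within the spawn plane's bounds, currently identical for every minigame type.
; The look input's sprite movement has no location wired yet.
; A debug-style key returns possession to the instigator and destroys the hand.
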(event Custom|spawnMinigame
  (bind _spawnplane (Variables|Default|GetspawnPlane))
  (bind (_origin _boxextent) (Collision|GetComponentBounds _spawnplane))
  (switch string (stale EventPossessed _output_get)
    (:Square%20Hole
      _)
    (:Tuck
      _)
    (:Stack
      _))
  (Game|SpawnActorfromClass "/Game/Blueprints/Minigames/SquareHole/BP_SH_grabber.BP_SH_grabber_C" (Math|Transform|MakeTransform (Math|Random|RandomPointinBoundingBox _origin _boxextent) "0, 0, 0" "0.100000,0.100000,0.100000") "Undefined" "MultiplyWithRoot" 0 0))

(event Input|EnhancedActionEvents|EnhancedInputActionIA_look
  (params (ActionValue :type Vector%202D%20Structure) (ElapsedSeconds :type Float%20%28double-precision%29) (TriggeredSeconds :type Float%20%28double-precision%29) (InputAction :type Input%20Action%20Object%20Reference :default "/Game/Blueprints/Input/IA_look.IA_look"))
  (Transformation|SetWorldLocation (Variables|Default|GetPaperSprite) (Math|Vector|MakeVector 0.0 0.0 0.0) false false))

(event EventPossessed
  (params (NewController :type Controller%20Object%20Reference))
  (Variables|Default|SetisPoss true)
  (bind _asbp_player_character (Utilities|Casting|CastToBP_playerCharacter (Game|GetInstigator)))
  (Variables|Default|SetAs%20BP%20Player%20Character _asbp_player_character)
  (bind _output_get (Variables|Default|SetcurMinigame (.OutItem (Utilities|Array|Random (Variables|Default|Getminigames)))))
  (CallFunction|SpawnMinigame))

(event Input|KeyboardEvents|Ö
  (params (Key :type Key%20Structure :default "None"))
  (:Pressed
    (Pawn|Possess (Game|GetPlayerController 0) (Game|GetInstigator))
    (Actor|DestroyActor)))

(fn ConstructionScript)