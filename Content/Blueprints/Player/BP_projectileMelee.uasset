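; BP_projectileMelee is a thrown pillow projectile that damages enemies and turns back into a pickup on impact.
; Tick spins it around its roll axis while it exists.
; Its sphere overlap subtracts Dmg from a BP_enemyPablo's clamped HP and destroys it.
; Pillow mesh overlaps with anything but the player destroy it and spawn a BP_pickupPillow, dislodged along the projectile's forward vector.
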(event OnComponentBeginOverlap(Sphere)
  (params (OverlappedComponent :type Primitive%20Component%20Object%20Reference) (OtherActor :type Actor%20Object%20Reference) (OtherComp :type Primitive%20Component%20Object%20Reference) (OtherBodyIndex :type Integer) (bFromSweep :type Boolean) (SweepResult :type Hit%20Result%20Structure%20%28by%20ref%29))
  (bind _asbp_enemy_pablo (Utilities|Casting|CastToBP_enemyPablo OtherActor))
  (Variables|/Game/Blueprints/Enemies/BP_enemyPablo.BP_enemyPablo_C|SethpCur _asbp_enemy_pablo (Math|Integer|Clamp(Integer) (- (Variables|/Game/Blueprints/Enemies/BP_enemyPablo.BP_enemyPablo_C|GethpCur _asbp_enemy_pablo) (Variables|Default|Getdmg)) 0 (Variables|/Game/Blueprints/Enemies/BP_enemyPablo.BP_enemyPablo_C|GethpMax _asbp_enemy_pablo)))
  (Actor|DestroyActor))

(event OnComponentBeginOverlap(pillow_single)
  (params (OverlappedComponent :type Primitive%20Component%20Object%20Reference) (OtherActor :type Actor%20Object%20Reference) (OtherComp :type Primitive%20Component%20Object%20Reference) (OtherBodyIndex :type Integer) (bFromSweep :type Boolean) (SweepResult :type Hit%20Result%20Structure%20%28by%20ref%29))
  (if (!= OtherActor self)
    (Utilities|Casting|CastToBP_playerCharacter OtherActor
      (:CastFailed
        (Actor|DestroyActor)
        (bind _returnvalue (Game|SpawnActorfromClass "/Game/Blueprints/Player/BP_pickupPillow.BP_pickupPillow_C" (Math|Transform|MakeTransform (Transformation|GetActorLocation) "0, 0, 0" "1.000000,1.000000,1.000000") "Undefined" "MultiplyWithRoot" 0 0))
        (Variables|/Game/Blueprints/Player/BP_pickupPillow.BP_pickupPillow_C|SetvecDislodge _returnvalue (Transformation|GetActorForwardVector))
        (Default|Dislodge _returnvalue)))))

(event EventTick
  (params (DeltaSeconds :type Float%20%28single-precision%29))
  (bind _returnvalue (Transformation|GetActorRotation))
  (Transformation|SetActorRotation (Math|Rotator|MakeRotator (+ (.roll _returnvalue) 15.0) (.pitch _returnvalue) (.yaw _returnvalue))))

(fn ConstructionScript)