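; BP_melee is a short-lived melee hitbox for the player's punch that destroys itself 0.3 seconds after spawning.
; Each tick it snaps to a point in front of the player along the camera's forward vector, matching the character's rotation.
; Its box overlap damages BP_enemyPablo, updates its HP and destroys the hitbox.
; It also sets BP_Tunnel as blocked and calls BePunched on BP_pillowFort.
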(event OnComponentBeginOverlap(Box)
  (params (OverlappedComponent :type Primitive%20Component%20Object%20Reference) (OtherActor :type Actor%20Object%20Reference) (OtherComp :type Primitive%20Component%20Object%20Reference) (OtherBodyIndex :type Integer) (bFromSweep :type Boolean) (SweepResult :type Hit%20Result%20Structure%20%28by%20ref%29))
  (Utilities|FlowControl|Sequence
    (:then_0
      (bind _asbp_enemy_pablo (Utilities|Casting|CastToBP_enemyPablo OtherActor))
      (Variables|/Game/Blueprints/Enemies/BP_enemyPablo.BP_enemyPablo_C|SethpCur _asbp_enemy_pablo (- (Variables|/Game/Blueprints/Enemies/BP_enemyPablo.BP_enemyPablo_C|GethpCur _asbp_enemy_pablo) (Variables|Default|Getdmg)))
      (Default|UpdateHP _asbp_enemy_pablo)
      (Actor|DestroyActor))
    (:then_1
      (bind _asbp_tunnel (Utilities|Casting|CastToBP_Tunnel OtherActor))
      (Variables|/Game/Blueprints/Level/BP_Tunnel.BP_Tunnel_C|SettunnelBlocked _asbp_tunnel true))
    (:then_2
      (bind _asbp_pillow_fort (Utilities|Casting|CastToBP_pillowFort OtherActor))
      (Default|BePunched _asbp_pillow_fort))))

(event EventBeginPlay
  (bind _asbp_player_character (Utilities|Casting|CastToBP_playerCharacter (Game|GetPlayerCharacter 0)))
  (Variables|Default|SetAs%20BP%20Player%20Character _asbp_player_character)
  (Utilities|FlowControl|Delay 0.3)
  (Actor|DestroyActor))

(event EventTick
  (params (DeltaSeconds :type Float%20%28single-precision%29))
  (bind _as_bp_player_character (Variables|Default|GetAs%20BP%20Player%20Character))
  (Transformation|SetActorLocationAndRotation (+ (Transformation|GetActorLocation _as_bp_player_character) (* 100 (Math|Vector|GetForwardVector (Variables|/Game/Blueprints/Player/BP_playerCharacter.BP_playerCharacter_C|GetCamera _as_bp_player_character)))) (Transformation|GetActorRotation _as_bp_player_character)))

(fn ConstructionScript)