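; Pillow ammo pickup that adds one to the player character's AmmoPillow on sphere overlap, then destroys itself.
; On spawn it teleports back along VecDislodge, then polls velocity each tick until the actor comes to rest.
; It then stores the resting height and restarts a Timeline endlessly to spin the pillow and bob the actor around that height.
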(event OnComponentBeginOverlap(Sphere)
  (params (OverlappedComponent :type Primitive%20Component%20Object%20Reference) (OtherActor :type Actor%20Object%20Reference) (OtherComp :type Primitive%20Component%20Object%20Reference) (OtherBodyIndex :type Integer) (bFromSweep :type Boolean) (SweepResult :type Hit%20Result%20Structure%20%28by%20ref%29))
  (Utilities|FlowControl|DelayUntilNextTick)
  (bind _asbp_player_character (Utilities|Casting|CastToBP_playerCharacter OtherActor))
  (Math|Integer|IncrementInt (Variables|/Game/Blueprints/Player/BP_playerCharacter.BP_playerCharacter_C|GetammoPillow _asbp_player_character)
    (:%20%20
      (Actor|DestroyActor))))

(event Custom|Dislodge
  (Transformation|SetActorLocation (- (Transformation|GetActorLocation) (* 80 (Variables|Default|GetvecDislodge))) false false)
  (if (> (Math|Vector|Distance(Vector) (Transformation|GetVelocity) "0, 0, 0") 1.0) :!label _label
    (Utilities|FlowControl|DelayUntilNextTick)
    (goto _label)
    (else
      (Variables|Default|SetzO (.z (Transformation|GetActorLocation)))
      (CallFunction|Bounce))))

(event Custom|Bounce
  (bind _returnvalue (Transformation|GetActorLocation))
  (bind _pillow_single (Variables|Default|Getpillow_single))
  (bind _returnvalue_2 (Transformation|GetWorldRotation _pillow_single))
  (bind _bounce (Timeline|Timeline PlayFromStart)
    (:Update
      (Transformation|SetWorldRotation _pillow_single (Math|Rotator|MakeRotator (.roll _returnvalue_2) (.pitch _returnvalue_2) (+ 3.0 (.yaw _returnvalue_2))) false false)
      (Transformation|SetActorLocation (Math|Vector|MakeVector (.x _returnvalue) (.y _returnvalue) (+ (* _bounce 2e+01) (Variables|Default|GetzO))) false false))
    (:Finished
      (Timeline|Timeline PlayFromStart))))

(event EventBeginPlay
  (Utilities|FlowControl|DelayUntilNextTick)
  (CallFunction|Dislodge))

(fn ConstructionScript)