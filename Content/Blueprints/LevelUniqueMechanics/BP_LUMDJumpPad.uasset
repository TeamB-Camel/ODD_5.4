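; Jump pad that grants the player character a double jump on overlap, then recharges before it can be used again.
; On use it switches its plane material to the off color and waits through a delay.
; A per-tick counter loop then blinks the color through a FlipFlop, so timing follows frame rate, and re-arms the pad on the on color.
; BeginPlay rescales both colors from 0-255 values.
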(event Collision|EventActorBeginOverlap
  (params (OtherActor :type Actor%20Object%20Reference))
  (bind _plane (Variables|Default|GetPlane))
  (bind _asbp_player_character (Utilities|Casting|CastToBP_playerCharacter OtherActor))
  (if (Variables|Default|GetcanBoost)
    (Default|GetDoubleJump _asbp_player_character)
    (Variables|Default|SetcanBoost false)
    (Rendering|Material|SetVectorParameterValueonMaterials (Variables|Default|GetPlane) "Color" (Variables|Default|GetcolorOff))
    (Utilities|FlowControl|Delay 3.0)
    (Utilities|FlowControl|DelayUntilNextTick :!label _label)
    (bind _result (Math|Float|IncrementFloat (Variables|Default|GetblinkTimer))
      (:%20%20
        (if (== (- (/ _result 1e+01) (Math|Float|Floor (/ _result 1e+01))) 0.0)
          (Utilities|FlowControl|FlipFlop
            (:A
              (Rendering|Material|SetVectorParameterValueonMaterials _plane "Color" (Variables|Default|GetcolorOn))
              (if (>= (Variables|Default|GetblinkTimer) 1.2e+02)
                (Variables|Default|SetblinkTimer 0.0)
                (Variables|Default|SetcanBoost true)
                (else
                  (goto _label))))
            (:B
              (Rendering|Material|SetVectorParameterValueonMaterials _plane "Color" (Variables|Default|GetcolorOff))
              (goto _label)))
          (else
            (goto _label)))))))

(event EventBeginPlay
  (Variables|Default|SetcolorOn (/ (Variables|Default|GetcolorOn) 255))
  (Variables|Default|SetcolorOff (/ (Variables|Default|GetcolorOff) 255))
  (Rendering|Material|SetVectorParameterValueonMaterials (Variables|Default|GetPlane) "Color" (Variables|Default|GetcolorOn)))

(fn ConstructionScript)