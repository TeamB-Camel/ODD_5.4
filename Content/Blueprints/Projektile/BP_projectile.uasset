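; BP_projectile is a projectile actor that damages BP_enemyPablo enemies when its Cube component begins an overlap.
; It reads PistolDmg from the player character, subtracts it from the enemy's HpCur, then destroys itself.
; An enemy whose HP drops to zero or below is destroyed directly by the projectile.
; Other overlaps only print a debug string and leave the projectile alive.
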(event OnComponentBeginOverlap(Cube)
  (params (OverlappedComponent :type Primitive%20Component%20Object%20Reference) (OtherActor :type Actor%20Object%20Reference) (OtherComp :type Primitive%20Component%20Object%20Reference) (OtherBodyIndex :type Integer) (bFromSweep :type Boolean) (SweepResult :type Hit%20Result%20Structure%20%28by%20ref%29))
  (Development|PrintString "Ouchie!" true true "(R=0.000000,G=0.660000,B=1.000000,A=1.000000)" 2.0 "enemyHit")
  (bind _asbp_player_character (Utilities|Casting|CastToBP_playerCharacter (Game|Player|GetPlayerPawn 0)))
  (bind _asbp_enemy_pablo (Utilities|Casting|CastToBP_enemyPablo OtherActor)
    (:then
      (Variables|/Game/Blueprints/Enemies/BP_enemyPablo.BP_enemyPablo_C|SethpCur _asbp_enemy_pablo (- (Variables|/Game/Blueprints/Enemies/BP_enemyPablo.BP_enemyPablo_C|GethpCur _asbp_enemy_pablo) (Variables|/Game/Blueprints/Player/BP_playerCharacter.BP_playerCharacter_C|GetpistolDmg _asbp_player_character)))
      (Actor|DestroyActor)
      (if (<= (Variables|/Game/Blueprints/Enemies/BP_enemyPablo.BP_enemyPablo_C|GethpCur _asbp_enemy_pablo) 0)
        (Actor|DestroyActor _asbp_enemy_pablo)))
    (:CastFailed
      (Development|PrintString "Hello"))))

(fn ConstructionScript)