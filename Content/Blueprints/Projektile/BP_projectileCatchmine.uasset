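; BP_projectileCatchmine is a thrown catch-mine projectile that turns into a placed mine where it lands.
; It picks a random rotation rate on BeginPlay and spins its sphere every tick during flight.
; On the sphere's first hit, it spawns a BP_instanceCatchmine at the impact point, oriented along the surface normal, then destroys itself.
; The overlap handler has no effect.
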(event OnComponentHit(Sphere)
  (params (HitComponent :type Primitive%20Component%20Object%20Reference) (OtherActor :type Actor%20Object%20Reference) (OtherComp :type Primitive%20Component%20Object%20Reference) (NormalImpulse :type Vector :default "0, 0, 0") (Hit :type Hit%20Result%20Structure%20%28by%20ref%29))
  (Game|SpawnActorfromClass "/Game/Blueprints/Projektile/BP_instanceCatchmine.BP_instanceCatchmine_C" (Math|Transform|MakeTransform (.location Hit) (Math|Rotator|FindLookatRotation (.location Hit) (+ (.location Hit) (.normal Hit))) "1.000000,1.000000,1.000000") "Undefined" "MultiplyWithRoot" 0 0)
  (Actor|DestroyActor))

(event EventBeginPlay
  (Variables|Default|SetrotFlight (Math|Vector|MakeVector (Math|Random|RandomFloatinRange 2.0 8.0) (Math|Random|RandomFloatinRange 2.0 8.0) (Math|Random|RandomFloatinRange 6.0 1e+01))))

(event Collision|EventActorBeginOverlap
  (params (OtherActor :type Actor%20Object%20Reference))
  (if (Actor|ActorHasTag OtherActor "None")
    _))

(event EventTick
  (params (DeltaSeconds :type Float%20%28single-precision%29))
  (bind _rotflight (Variables|Default|GetrotFlight))
  (Transformation|AddLocalRotation (Variables|Default|GetSphere) (Math|Rotator|MakeRotator (.x _rotflight) (.y _rotflight) (.z _rotflight)) false false))

(fn ConstructionScript)