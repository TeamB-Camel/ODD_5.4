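; BP_projectileRifle is a rifle projectile that damages BP_enemyPablo enemies on overlap.
; It destroys itself after a set Duration or on overlapping any actor other than BP_playerCharacter, which it ignores.
; On an enemy hit it subtracts DMG directly from the enemy's HpCur and destroys that enemy when health reaches zero or below, without using Unreal's damage system.
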(event EventBeginPlay
  (Utilities|FlowControl|Delay (Variables|Default|GetDuration))
  (Actor|DestroyActor)
  (Development|PrintString "Uff"))

(event Collision|EventActorBeginOverlap
  (params (OtherActor :type Actor%20Object%20Reference))
  (Utilities|Casting|CastToBP_playerCharacter OtherActor
    (:CastFailed
      (bind _asbp_enemy_pablo (Utilities|Casting|CastToBP_enemyPablo OtherActor)
        (:then
          (Variables|/Game/Blueprints/Enemies/BP_enemyPablo.BP_enemyPablo_C|SethpCur _asbp_enemy_pablo (- (Variables|/Game/Blueprints/Enemies/BP_enemyPablo.BP_enemyPablo_C|GethpCur _asbp_enemy_pablo) (Variables|Default|GetDMG)))
          (Actor|DestroyActor)
          (if (<= (Variables|/Game/Blueprints/Enemies/BP_enemyPablo.BP_enemyPablo_C|GethpCur _asbp_enemy_pablo) 0.0)
            (Actor|DestroyActor _asbp_enemy_pablo)))
        (:CastFailed
          (Actor|DestroyActor))))))

(fn ConstructionScript)