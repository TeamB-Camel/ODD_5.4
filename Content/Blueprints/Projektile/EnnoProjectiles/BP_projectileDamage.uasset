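; BP_projectileDamage is a projectile that damages BP_enemyPablo enemies on overlap.
; It subtracts its Damage from the enemy's current HP, calls UpdateHP, and destroys itself on overlapping anything except BP_playerCharacter.
; BeginPlay only caches the player character; disconnected nodes that would read damage, speed and lifetime from the player's weapon map never run.
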(event EventBeginPlay
  (bind _asbp_player_character (Utilities|Casting|CastToBP_playerCharacter (Game|GetPlayerCharacter 0)))
  (bind _output_get (Variables|Default|SetAs%20BP%20Player%20Character _asbp_player_character)))

(event Collision|EventActorBeginOverlap
  (params (OtherActor :type Actor%20Object%20Reference))
  (Utilities|Casting|CastToBP_playerCharacter OtherActor
    (:CastFailed
      (bind _asbp_enemy_pablo (Utilities|Casting|CastToBP_enemyPablo OtherActor)
        (:then
          (Variables|/Game/Blueprints/Enemies/BP_enemyPablo.BP_enemyPablo_C|SethpCur _asbp_enemy_pablo (- (Variables|/Game/Blueprints/Enemies/BP_enemyPablo.BP_enemyPablo_C|GethpCur _asbp_enemy_pablo) (Variables|Default|GetDamage)))
          (Default|UpdateHP _asbp_enemy_pablo))
        (:CastFailed
          _))
      (Actor|DestroyActor))))

(fn ConstructionScript)