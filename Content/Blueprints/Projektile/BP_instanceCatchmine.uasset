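; BP_instanceCatchmine is a placed catch mine that grabs a single BP_enemyPablo that comes within range, then destroys itself.
; Tick scans all those enemies until one is within DistCatch, then Catch launches it toward the mine each tick while moving Sphere onto its sprite.
; Inside DistStick, Hold pins the target's XY to the mine for IntervalHold ticks before Release.
; Both phases loop through DelayUntilNextTick.
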(event Custom|catch
  (bind _returnvalue (Transformation|GetActorLocation))
  (bind _catchtarget (Variables|Default|GetcatchTarget))
  (bind _returnvalue_2 (Transformation|GetActorLocation _catchtarget))
  (bind _returnvalue_3 (Math|Vector|Distance(Vector) _returnvalue _returnvalue_2))
  (if (> _returnvalue_3 (Variables|Default|GetdistStick)) :!label _label
    (Character|LaunchCharacter _catchtarget (* (Math|Vector|Normalize (- _returnvalue _returnvalue_2)) (Variables|Default|Getpullspd)) false false)
    (Transformation|SetWorldLocation (Variables|Default|GetSphere) (Transformation|GetWorldLocation (Variables|/Game/Blueprints/Enemies/BP_enemyPablo.BP_enemyPablo_C|GetPaperSprite (Variables|Default|GetcatchTarget))) false false)
    (Development|PrintString (Utilities|String|ToString(Float) _returnvalue_3))
    (Utilities|FlowControl|DelayUntilNextTick)
    (goto _label)
    (else
      (CallFunction|Hold))))

(event Custom|hold
  (bind _returnvalue (Transformation|GetActorLocation))
  (bind _tickshold (Variables|Default|GetticksHold))
  (bind _catchtarget (Variables|Default|GetcatchTarget))
  (Transformation|SetActorLocation _catchtarget (Math|Vector|MakeVector (.x _returnvalue) (.y _returnvalue) (.z (Transformation|GetActorLocation _catchtarget))) false false :!label _label)
  (Math|Integer|IncrementInt _tickshold
    (:%20%20
      (if (== _tickshold (Variables|Default|GetintervalHold))
        (CallFunction|Release)
        (else
          (Utilities|FlowControl|DelayUntilNextTick)
          (goto _label))))))

(event Custom|release
  (Actor|DestroyActor))

(event EventTick
  (params (DeltaSeconds :type Float%20%28single-precision%29))
  (if (not (Variables|Default|GetisCatching))
    (bind _outactors (Actor|GetAllActorsOfClass "/Game/Blueprints/Enemies/BP_enemyPablo.BP_enemyPablo_C"))
    (bind _array_element (Utilities|Array|ForEachLoopwithBreak _outactors :!label _label)
      (:LoopBody
        (if (< (Math|Vector|Distance(Vector) (Transformation|GetActorLocation _array_element) (Transformation|GetActorLocation)) (Variables|Default|GetdistCatch))
          (Variables|Default|SetcatchTarget _array_element)
          (CallFunction|Catch)
          (Variables|Default|SetisCatching true)
          (goto _label Break))))))

(fn ConstructionScript)