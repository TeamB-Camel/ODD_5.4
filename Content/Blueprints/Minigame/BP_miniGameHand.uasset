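; Possessable hand pawn that runs a shape-sorting minigame, then returns control to the player character that spawned it.
; On possession it picks a random minigame type, though all three cases spawn BP_SH_grabber.
; Look input moves the hand; shoot box-traces downward to attach the shape, then matches the hole's component name against CurShape.
; A correct match, or the Ö key, destroys minigame and hand and repossesses the instigator.
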(event Custom|spawnMinigame
  (switch string (stale EventPossessed _output_get)
    (:Square%20Hole
      _)
    (:Tuck
      _)
    (:Stack
      _))
  (bind _returnvalue (Game|SpawnActorfromClass "/Game/Blueprints/Minigame/SquareHole/BP_SH_grabber.BP_SH_grabber_C" (Math|Transform|MakeTransform (Transformation|GetWorldLocation (Variables|Default|GetspawnPoint)) (Transformation|GetActorRotation) "0.100000,0.100000,0.100000") "Undefined" "MultiplyWithRoot" 0 self))
  (Variables|Default|SetignoreList (Utilities|Array|MakeArray _returnvalue)))

(event Custom|destroyMinigame
  (params (mingameObject :type Actor%20Object%20Reference))
  (Actor|DestroyActor mingameObject)
  (Pawn|Possess (Game|GetPlayerController 0) (Game|GetInstigator))
  (Actor|DestroyActor))

(event Input|EnhancedActionEvents|EnhancedInputActionIA_look
  (params (ActionValue :type Vector%202D%20Structure) (ElapsedSeconds :type Float%20%28double-precision%29) (TriggeredSeconds :type Float%20%28double-precision%29) (InputAction :type Input%20Action%20Object%20Reference :default "/Game/Blueprints/Input/IA_look.IA_look"))
  (bind (_x _y) (Math|Vector2D|BreakVector2D ActionValue))
  (bind _returnvalue (* _y -1.0))
  (Class|SceneComponent|AddLocalTransform (Variables|Default|GetPaperSprite) (Math|Transform|MakeTransform (Math|Vector|MakeVector _returnvalue 0.0 _x) "0, 0, 0" "2.750000,1.000000,0.250000") false false)
  (Class|SceneComponent|AddLocalTransform (Variables|Default|GetgrabPoint) (Math|Transform|MakeTransform (Math|Vector|MakeVector _returnvalue _x 0.0) "0, 0, 0" "1.000000,1.000000,1.000000") false false))

(event Input|EnhancedActionEvents|EnhancedInputActionIA_shoot
  (params (ActionValue :type Boolean) (ElapsedSeconds :type Float%20%28double-precision%29) (TriggeredSeconds :type Float%20%28double-precision%29) (InputAction :type Input%20Action%20Object%20Reference :default "/Game/Blueprints/Input/IA_shoot.IA_shoot"))
  (bind _grabpoint (Variables|Default|GetgrabPoint))
  (bind _returnvalue (Transformation|GetWorldLocation _grabpoint))
  (bind _returnvalue_2 (- (.z _returnvalue) 5e+01))
  (bind _returnvalue_3 (Math|Vector|MakeVector (.x _returnvalue) (.y _returnvalue) _returnvalue_2))
  (bind (_x _y _z) (Math|Vector|BreakVector _returnvalue_3))
  (bind _returnvalue_4 (- _z 1e+03))
  (bind _returnvalue_5 (Math|Vector|MakeVector _x _y _returnvalue_4))
  (:Started
    (if (Variables|Default|GetisHold)
      (bind _outhit (Collision|BoxTraceByChannel _returnvalue_3 _returnvalue_5 "10.000000,10.000000,10.000000" "0, 0, 0" "TraceTypeQuery1" false 0 "ForDuration"))
      (bind _asbp_sh_grabber (Utilities|Casting|CastToBP_SH_grabber (.HitActor (Collision|BreakHitResult _outhit))))
      (Development|PrintString (Utilities|GetObjectName (.HitComponent (Collision|BreakHitResult _outhit))))
      (switch string (Utilities|GetObjectName (.HitComponent (Collision|BreakHitResult _outhit)))
        (:cubeHole
          (if (Utilities|Enum|Equal(Enum) (Variables|/Game/Blueprints/Minigame/SquareHole/BP_SH_grabber.BP_SH_grabber_C|GetcurShape _asbp_sh_grabber) "Square")
            (Components|DestroyComponent (.HitComponent (Collision|BreakHitResult (stale _outhit_2))))
            (CallFunction|DestroyMinigame _asbp_sh_grabber :!label _label)))
        (:sphereHole
          (if (Utilities|Enum|Equal(Enum) (Variables|/Game/Blueprints/Minigame/SquareHole/BP_SH_grabber.BP_SH_grabber_C|GetcurShape _asbp_sh_grabber) "Sphere")
            (Components|DestroyComponent (.HitComponent (Collision|BreakHitResult (stale _outhit_2))))
            (goto _label)))
        (:triangleHole
          (if (Utilities|Enum|Equal(Enum) (Variables|/Game/Blueprints/Minigame/SquareHole/BP_SH_grabber.BP_SH_grabber_C|GetcurShape _asbp_sh_grabber) "Triangle")
            (Components|DestroyComponent (.HitComponent (Collision|BreakHitResult (stale _outhit_2))))
            (goto _label)))
        (:starHole
          (if (Utilities|Enum|Equal(Enum) (Variables|/Game/Blueprints/Minigame/SquareHole/BP_SH_grabber.BP_SH_grabber_C|GetcurShape _asbp_sh_grabber) "Star")
            (Components|DestroyComponent (.HitComponent (Collision|BreakHitResult (stale _outhit_2))))
            (goto _label))))
      (else
        (bind _outhit_2 (Collision|BoxTraceByChannel _returnvalue_3 _returnvalue_5 "10.000000,10.000000,0.000000" "0, 0, 0" "TraceTypeQuery1" false 0 "ForDuration"))
        (bind _asbp_sh_grabber_2 (Utilities|Casting|CastToBP_SH_grabber (.HitActor (Collision|BreakHitResult _outhit_2))))
        (if (== (Variables|/Game/Blueprints/Minigame/SquareHole/BP_SH_grabber.BP_SH_grabber_C|GetStaticMesh _asbp_sh_grabber_2) (.HitComponent (Collision|BreakHitResult _outhit_2)))
          (Transformation|AttachComponentToComponent (.HitComponent (Collision|BreakHitResult _outhit_2)) (Variables|Default|GetgrabPoint) "None" "SnapToTarget" "KeepRelative" "KeepWorld" true)
          (Variables|Default|SetisHold true))))))

(event EventPossessed
  (params (NewController :type Controller%20Object%20Reference))
  (Variables|Default|SetisPoss true)
  (bind _asbp_player_character (Utilities|Casting|CastToBP_playerCharacter (Game|GetInstigator)))
  (Variables|Default|SetAs%20BP%20Player%20Character _asbp_player_character)
  (bind _output_get (Variables|Default|SetcurMinigame (.OutItem (Utilities|Array|Random (Variables|Default|Getminigames)))))
  (CallFunction|SpawnMinigame))

(event Input|KeyboardEvents|Ö
  (params (Key :type Key%20Structure :default "None"))
  (:Pressed
    (bind _outactors (Actor|GetAllActorsOfClass "/Game/Blueprints/Minigame/SquareHole/BP_SH_grabber.BP_SH_grabber_C"))
    (for _array_element _outactors
      (CallFunction|DestroyMinigame _array_element))))

(fn ConstructionScript)