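; BP_SH_grabber is an actor for the SquareHole minigame that sets up a random shape and scatters four shape holes.
; On BeginPlay it picks a square, triangle, circle or star, setting the mesh and CurShape name to match.
; It then randomizes each hole's relative XY position, looping back to re-roll while another hole's origin lies inside its padded bounds.
; No grab logic is present, and Tick is empty.
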(event EventBeginPlay
  (bind _staticmesh (Variables|Default|GetStaticMesh))
  (bind _trianglehole (Variables|Default|GettriangleHole))
  (bind _starhole (Variables|Default|GetstarHole))
  (bind _cubehole (Variables|Default|GetcubeHole))
  (bind _spherehole (Variables|Default|GetsphereHole))
  (bind _array (Utilities|Array|MakeArray _spherehole _trianglehole _starhole _cubehole))
  (Utilities|FlowControl|Sequence
    (:then_0
      (switch string (.OutItem (Utilities|Array|Random (Variables|Default|GetobjectShape)))
        (:Square
          (Components|StaticMesh|SetStaticMesh _staticmesh "/Engine/BasicShapes/Cube.Cube")
          (Variables|Default|SetcurShape "Square"))
        (:Triangle
          (Components|StaticMesh|SetStaticMesh _staticmesh "/Engine/VREditor/BasicMeshes/SM_Pyramid_01.SM_Pyramid_01")
          (Variables|Default|SetcurShape "Triangle"))
        (:Circle
          (Components|StaticMesh|SetStaticMesh _staticmesh "/Engine/BasicShapes/Cylinder.Cylinder")
          (Variables|Default|SetcurShape "Sphere"))
        (:Star
          (Components|StaticMesh|SetStaticMesh _staticmesh "/ControlRig/Controls/ControlRig_Star4_solid.ControlRig_Star4_solid")
          (Variables|Default|SetcurShape "Star"))))
    (:then_1
      (for _array_element _array
        (Transformation|SetRelativeLocation _array_element (Math|Vector|MakeVector (Math|Random|RandomFloatinRange -1e+03 1e+03) (Math|Random|RandomFloatinRange -1e+03 1e+03) 1.0) false false :!label _label)
        (for _array_element_2 _array
          (if (!= _array_element_2 _array_element)
            (if (Math|Geometry|IsPointinBox (Transformation|GetWorldLocation _array_element_2) (.Origin (Collision|GetComponentBounds _array_element)) (Math|Vector|MakeVector (+ (.x (.BoxExtent (Collision|GetComponentBounds _array_element))) 25.0) (+ (.y (.BoxExtent (Collision|GetComponentBounds _array_element))) 25.0) (.z (.BoxExtent (Collision|GetComponentBounds _array_element)))))
              (goto _label))))))))

(event EventTick
  (params (DeltaSeconds :type Float%20%28single-precision%29)))

(fn ConstructionScript)