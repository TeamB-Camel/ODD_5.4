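; Player weapon projectile that damages BP_enemyPablo enemies it overlaps.
; On BeginPlay it looks up the player's current weapon in MapWeapons, copies damage and speed from its projectile data, prints the damage, and destroys itself after that data's lifetime.
; Overlapping an enemy subtracts Damage from its HpCur and calls UpdateHP.
; Any overlap destroys the projectile, provided the player cast in BeginPlay is not involved.
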(event EventBeginPlay
  (bind _projectilemovement (Variables|Default|GetProjectileMovement))
  (bind _asbp_player_character (Utilities|Casting|CastToBP_playerCharacter (Game|GetPlayerCharacter 0)))
  (bind _output_get (Variables|Default|SetAs%20BP%20Player%20Character _asbp_player_character))
  (bind _output_get_2 (Variables|Default|SetDamage (.damage (Utilities|Struct|BreakStruct_projectileData (.dataProjectile (Utilities|Struct|BreakStruct_weaponData (.Value (Utilities|Map|Find (Variables|/Game/Blueprints/Player/BP_playerCharacter.BP_playerCharacter_C|GetmapWeapons _output_get) (Variables|/Game/Blueprints/Player/BP_playerCharacter.BP_playerCharacter_C|Getweapon _output_get)))))))))
  (Variables|/Script/Engine.ProjectileMovementComponent|SetMaxSpeed _projectilemovement (.spdProjectile (Utilities|Struct|BreakStruct_projectileData (.dataProjectile (Utilities|Struct|BreakStruct_weaponData (.Value (Utilities|Map|Find (Variables|/Game/Blueprints/Player/BP_playerCharacter.BP_playerCharacter_C|GetmapWeapons _output_get) (Variables|/Game/Blueprints/Player/BP_playerCharacter.BP_playerCharacter_C|Getweapon _output_get))))))))
  (Variables|/Script/Engine.ProjectileMovementComponent|SetInitialSpeed _projectilemovement (.spdProjectile (Utilities|Struct|BreakStruct_projectileData (.dataProjectile (Utilities|Struct|BreakStruct_weaponData (.Value (Utilities|Map|Find (Variables|/Game/Blueprints/Player/BP_playerCharacter.BP_playerCharacter_C|GetmapWeapons _output_get) (Variables|/Game/Blueprints/Player/BP_playerCharacter.BP_playerCharacter_C|Getweapon _output_get))))))))
  (Development|PrintString (Utilities|String|ToString(Float) _output_get_2))
  (Utilities|FlowControl|Delay (.lifetime (Utilities|Struct|BreakStruct_projectileData (.dataProjectile (Utilities|Struct|BreakStruct_weaponData (.Value (Utilities|Map|Find (Variables|/Game/Blueprints/Player/BP_playerCharacter.BP_playerCharacter_C|GetmapWeapons _output_get) (Variables|/Game/Blueprints/Player/BP_playerCharacter.BP_playerCharacter_C|Getweapon _output_get))))))))
  (Actor|DestroyActor))

(event Collision|EventActorBeginOverlap
  (params (OtherActor :type Actor%20Object%20Reference))
  (bind _asbp_enemy_pablo (Utilities|Casting|CastToBP_enemyPablo OtherActor)
    (:then
      (Variables|/Game/Blueprints/Enemies/BP_enemyPablo.BP_enemyPablo_C|SethpCur _asbp_enemy_pablo (- (Variables|/Game/Blueprints/Enemies/BP_enemyPablo.BP_enemyPablo_C|GethpCur _asbp_enemy_pablo) (Variables|Default|GetDamage)))
      (Default|UpdateHP _asbp_enemy_pablo))
    (:CastFailed
      _))
  (Actor|DestroyActor))

(fn ConstructionScript)