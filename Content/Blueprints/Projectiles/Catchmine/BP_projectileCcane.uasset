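; Spinning cane projectile from the Catchmine set that applies a stacking slow modifier to BP_enemyPablo enemies on overlap.
; It starts at a random yaw, rotates by a fixed step each tick independent of delta time, and expires after two seconds.
; Each enemy overlap decrements ModSlowed while it is above a floor threshold, then destroys the projectile; other actors are ignored.
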(event OnComponentBeginOverlap(Sphere)
  (params (OverlappedComponent :type Primitive%20Component%20Object%20Reference) (OtherActor :type Actor%20Object%20Reference) (OtherComp :type Primitive%20Component%20Object%20Reference) (OtherBodyIndex :type Integer) (bFromSweep :type Boolean) (SweepResult :type Hit%20Result%20Structure%20%28by%20ref%29))
  (bind _asbp_enemy_pablo (Utilities|Casting|CastToBP_enemyPablo OtherActor))
  (if (> (Variables|/Game/Blueprints/Enemies/BP_enemyPablo.BP_enemyPablo_C|GetmodSlowed _asbp_enemy_pablo) 0.2)
    (Variables|/Game/Blueprints/Enemies/BP_enemyPablo.BP_enemyPablo_C|SetmodSlowed _asbp_enemy_pablo (- (Variables|/Game/Blueprints/Enemies/BP_enemyPablo.BP_enemyPablo_C|GetmodSlowed _asbp_enemy_pablo) 0.1)))
  (Actor|DestroyActor))

(event EventTick
  (params (DeltaSeconds :type Float%20%28single-precision%29))
  (Transformation|AddLocalRotation (Variables|Components|GetprojectileCcane) "0.000000,12.000000,0.000000" false false))

(event EventBeginPlay
  (Transformation|AddLocalRotation (Variables|Components|GetprojectileCcane) (Math|Rotator|MakeRotator 0.0 0.0 (Math|Random|RandomFloatinRange 0.0 3.6e+02)) false false)
  (Utilities|FlowControl|Delay 2.0)
  (Actor|DestroyActor))

(fn ConstructionScript)