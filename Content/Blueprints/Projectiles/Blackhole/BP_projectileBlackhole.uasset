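; Black hole projectile that drags BP_enemyPablo enemies toward itself and destroys itself after a fixed delay.
; Each tick it yaws its Paper2D sprite to face the player, then scans all enemies of that class.
; Those inside RangeSuck are launched inward with a linear distance falloff that uses a hardcoded divisor rather than RangeSuck.
; Enemies within RangeStick are snapped to its center.
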(event EventTick
  (params (DeltaSeconds :type Float%20%28single-precision%29))
  (bind _returnvalue (Transformation|GetActorLocation))
  (Utilities|FlowControl|Sequence
    (:then_0
      ;[1 1 1] Rotation
      (Transformation|SetWorldRotation (Variables|Default|GetPaperSprite) (Math|Rotator|MakeRotator 0.0 0.0 (+ 9e+01 (.yaw (Math|Rotator|FindLookatRotation (Transformation|GetActorLocation) (Transformation|GetActorLocation (Game|Player|GetPlayerPawn 0)))))) false false))
    (:then_1
      ;[1 1 1] the succ
      (bind _outactors (Actor|GetAllActorsOfClass "/Game/Blueprints/Enemies/BP_enemyPablo.BP_enemyPablo_C"))
      (for _array_element _outactors
        (if (< (Math|Vector|Distance(Vector) (Transformation|GetActorLocation _array_element) _returnvalue) (Variables|Default|GetrangeSuck))
          (if (> (Math|Vector|Distance(Vector) (Transformation|GetActorLocation _array_element) _returnvalue) (Variables|Default|GetrangeStick))
            (Character|LaunchCharacter _array_element (* (* (Math|Vector|Normalize (- _returnvalue (Transformation|GetActorLocation _array_element))) (Variables|Default|GetfactorSuck)) (- 1.0 (/ (Math|Vector|Distance(Vector) (Transformation|GetActorLocation _array_element) _returnvalue) 2e+03))) false false)
            (else
              (Transformation|SetActorLocation _array_element _returnvalue false false))))))))

(event EventBeginPlay
  (Utilities|FlowControl|Delay 1e+01)
  (Actor|DestroyActor))

(fn ConstructionScript)