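; Portal projectile that spawns a BP_instancePortal where it hits, oriented along the surface normal, and expires after a short lifetime.
; On BeginPlay it counts all portal projectiles and placed portals, itself included, and turns blue when the total is odd.
; On hit, a blue projectile passes its color to the new portal and destroys itself; a non-blue one only spawns the portal.
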(event OnComponentHit(Sphere)
  (params (HitComponent :type Primitive%20Component%20Object%20Reference) (OtherActor :type Actor%20Object%20Reference) (OtherComp :type Primitive%20Component%20Object%20Reference) (NormalImpulse :type Vector :default "0, 0, 0") (Hit :type Hit%20Result%20Structure%20%28by%20ref%29))
  (bind _returnvalue (Game|SpawnActorfromClass "/Game/Blueprints/Projectiles/Blackhole/BP_instancePortal.BP_instancePortal_C" (Math|Transform|MakeTransform (.location Hit) (Math|Rotator|FindLookatRotation (.location Hit) (+ (.location Hit) (.normal Hit))) "1.000000,1.000000,1.000000") "Undefined" "MultiplyWithRoot" 0 0))
  (if (Variables|Default|Getblue)
    (Rendering|Material|SetVectorParameterValueonMaterials (Variables|/Game/Blueprints/Projectiles/Blackhole/BP_instancePortal.BP_instancePortal_C|GetSphere _returnvalue) "Color" "0.000000,0.000000,255.000000")
    (Actor|DestroyActor)))

(event EventBeginPlay
  (Utilities|FlowControl|Sequence
    (:then_0
      (bind _outactors (Actor|GetAllActorsOfClass "BP_projectilePortal_C"))
      (bind _outactors_2 (Actor|GetAllActorsOfClass "/Game/Blueprints/Projectiles/Blackhole/BP_instancePortal.BP_instancePortal_C"))
      (Variables|Default|SetportalsTotal (+ (Utilities|Array|Length _outactors) (Utilities|Array|Length _outactors_2))))
    (:then_1
      (if (== (Math|Integer|%(Integer) (Variables|Default|GetportalsTotal) 2) 1)
        (Variables|Default|Setblue true)
        (Rendering|Material|SetVectorParameterValueonMaterials (Variables|Default|GetSphere) "Color" "0.000000,0.000000,255.000000")))
    (:then_2
      (Utilities|FlowControl|Delay 5.0)
      (Actor|DestroyActor))))

(fn ConstructionScript)